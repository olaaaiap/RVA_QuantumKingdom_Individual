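; BP_Basic_Enemy is a basic enemy that dies to projectiles and damages the Olaia VR pawn on contact.
; All combat runs through actor overlap: a Projectile destroys both itself and the enemy, while an OlaiaVRPawn has its TakeDamage called.
; A short spawn-protection flag, cleared after a delay in BeginPlay, makes the enemy ignore overlaps right after it spawns.
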(event EventBeginPlay
  (Variables|Default|SetIsSpawnProtected true)
  (Utilities|FlowControl|Delay 0.5)
  (Variables|Default|SetIsSpawnProtected false))

(event Collision|EventActorBeginOverlap
  (params (OtherActor :type Actor%20Object%20Reference))
  (if (== (Variables|Default|GetIsSpawnProtected) false)
    (bind _asprojectile (Utilities|Casting|CastToProjectile OtherActor)
      (:then
        (Actor|DestroyActor _asprojectile)
        (Actor|DestroyActor))
      (:CastFailed
        (bind _asolaia_vrpawn (Utilities|Casting|CastToOlaiaVRPawn OtherActor))
        (Default|TakeDamage _asolaia_vrpawn)))))

(event EventTick
  (params (DeltaSeconds :type Float%20%28single-precision%29)))

(fn ConstructionScript)