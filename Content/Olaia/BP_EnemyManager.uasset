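; BP_EnemyManager spawns BP_Basic_Enemy in timed, escalating waves at random TargetPoints in the level.
; BeginPlay caches all TargetPoints, then chains Delays into waves of one, two and three enemies.
; SpawnEnemy picks a random point, spawns the enemy there and gives it its default controller.
; The final loop wraps a latent Delay, which ignores retriggers, so the three-enemy wave fires once rather than repeating.
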(event Custom|SpawnWave1
  (CallFunction|SpawnEnemy))

(event Custom|SpawnWave2
  (for _index (range 0 1)
    (CallFunction|SpawnEnemy)))

(event Custom|SpawnWave3
  (for _index (range 0 2)
    (CallFunction|SpawnEnemy)))

(event EventBeginPlay
  (bind _outactors (Actor|GetAllActorsOfClass "/Script/Engine.TargetPoint"))
  (for _array_element _outactors
    (Utilities|Array|Add (Variables|Default|GetSpawnPoints) _array_element))
  (Utilities|Time|SetTimerbyEvent (EventDispatchers|CreateEvent :!event Custom|SpawnWave1) 0.0)
  (Utilities|FlowControl|Delay 0.2)
  (CallFunction|SpawnWave1)
  (Utilities|FlowControl|Delay 15.0)
  (CallFunction|SpawnWave2)
  (Utilities|FlowControl|Delay 15.0)
  (CallFunction|SpawnWave2)
  (for _index (range 0 20)
    (Utilities|FlowControl|Delay 4e+01)
    (CallFunction|SpawnWave3)))

(event Collision|EventActorBeginOverlap
  (params (OtherActor :type Actor%20Object%20Reference)))

(event EventTick
  (params (DeltaSeconds :type Float%20%28single-precision%29)))

(fn ConstructionScript)

(fn SpawnEnemy
  (bind _returnvalue (Game|SpawnActorfromClass "/Game/Olaia/IA/BP_Basic_Enemy.BP_Basic_Enemy_C" (Transformation|GetActorTransform (Utilities|Array|Get(acopy) (Variables|Default|GetSpawnPoints) (Math|Random|RandomIntegerinRange 0 (- (Utilities|Array|Length (Variables|Default|GetSpawnPoints)) 1)))) "Undefined" "MultiplyWithRoot" 0 0))
  (bind _asbp_basic_enemy (Utilities|Casting|CastToBP_Basic_Enemy _returnvalue))
  (Utilities|IsValid _asbp_basic_enemy
    (:Is%20Valid
      (Pawn|SpawnDefaultController _asbp_basic_enemy))))